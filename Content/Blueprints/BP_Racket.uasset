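; Player paddle for an Arkanoid-style game that also runs the level flow, from HUD and pause menu to game-over and win screens.
; It moves with swept offsets, launches an attached ball, respawns it when lost, and supports bonus balls and timed twin-laser bursts.
; Lives and blocks components track progress via event dispatchers, loading lives and score from the game instance and saving them back when blocks die.
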(event `self.ReceiveBeginPlay`
  (`GameplayStatics.PlaySound2D` "/Game/Blueprints/Audio/S_MainMusic_Cue.S_MainMusic_Cue" 1.0 1.0 0.0 null null)
  (`self.InitializeSettings`)
  (`|ExecutionSequence`
    (:`then_0`
      (`WidgetBlueprintLibrary.SetInputMode_GameOnly` (`GameplayStatics.GetPlayerController` 0)))
    (:`then_1`
      (`self.BindsLivesComponent`)
      (`self.SpawnBall`)
      (bind _returnvalue (`|CreateWidget` "/Game/Blueprints/UI/W_Hud.W_Hud_C"))
      (`UserWidget.AddToViewport` _returnvalue 0)
      (set `self.Hud` _returnvalue)
      (for _array_element (`self.BlocksArray`)
        (add `/Game/Blueprints/BP_Block.OnBlockDead` _array_element (delegate `BlockDead`))))))

(event `BlockDead`
  (params (Score :type Integer))
  (`/Game/Blueprints/ActorComponents/BP_BlocksCounter.SubBlock` (`self.BP_BlocksCounter`) Score)
  (`self.BindsBlocksCounter`)
  (`self.SetGameInstance`))

(event `InputAxis|MoveRight`
  (params (AxisValue :type "Float (single-precision)"))
  ;[1 1 1] Racket Movement
  (if (< AxisValue 0.0)
    (`self.K2_AddActorWorldOffset` (`KismetMathLibrary.MakeVector` (* (`self.RacketSpeed`) -1.0)) true)))

(event `InputAxis|MoveRight`
  (params (AxisValue :type "Float (single-precision)"))
  ;[1 1 1] Racket Movement
  (if (> AxisValue 0.0)
    (`self.K2_AddActorWorldOffset` (`KismetMathLibrary.MakeVector` (`self.RacketSpeed`)) true)))

(event `InputAction|PushBall`
  (params (Key :type "Key Structure"))
  ;[1 1 1] Push the Ball
  (:`Pressed`
    (bind _playingball (`self.PlayingBall`)
      (:`then`
        (`self.K2_DetachFromActor` _playingball "KeepWorld" "KeepWorld" "KeepWorld")
        (`self.OnPushBall`))
      (:`else`))))

(event `InputAction|Exit`
  (params (Key :type "Key Structure"))
  (bind _returnvalue (`GameplayStatics.GetPlayerController` (`self.Player Index`)))
  (:`Pressed`
    (bind _returnvalue_2 (`|CreateWidget` "/Game/Blueprints/UI/W_PauseGame.W_PauseGame_C" _returnvalue))
    (`UserWidget.AddToViewport` _returnvalue_2 0)
    (`WidgetBlueprintLibrary.SetInputMode_UIOnlyEx` _returnvalue _returnvalue_2 "LockOnCapture")
    (set `PlayerController.bShowMouseCursor` true _returnvalue)
    (`GameplayStatics.SetGamePaused` true)))

(fn `BindsBlocksCounter`
  (add `/Game/Blueprints/ActorComponents/BP_BlocksCounter.OnBlocksEnd` (`self.BP_BlocksCounter`) (`|CreateDelegate` :!event `LevelCompleted`)))

(fn `BindsLivesComponent`
  (add `/Game/Blueprints/ActorComponents/BP_LivesComponent.OnLivesEnd` (`self.BP_LivesComponent`) (`|CreateDelegate` :!event `Game Over`)))

(fn `Game Over`
  (bind _returnvalue (`GameplayStatics.GetPlayerController` (`self.Player Index`)))
  (`Widget.SetVisibility` (`self.Hud`) "Collapsed")
  (bind _returnvalue_2 (`|CreateWidget` "/Game/Blueprints/UI/W_GameOver.W_GameOver_C" _returnvalue))
  (`UserWidget.AddToViewport` _returnvalue_2 0)
  (`WidgetBlueprintLibrary.SetInputMode_UIOnlyEx` _returnvalue _returnvalue_2 "LockOnCapture")
  (set `PlayerController.bShowMouseCursor` true _returnvalue)
  (`self.K2_DestroyActor`))

(fn `InitializeSettings`
  (bind _bp_blockscounter (`self.BP_BlocksCounter`))
  (bind _asgi_arkanoid_game_instance (cast `/Game/Blueprints/GI_ArkanoidGameInstance` (`GameplayStatics.GetGameInstance`)))
  (set `/Game/Blueprints/ActorComponents/BP_LivesComponent.Lives` (`/Game/Blueprints/GI_ArkanoidGameInstance.Lives` _asgi_arkanoid_game_instance) (`self.BP_LivesComponent`))
  (set `/Game/Blueprints/ActorComponents/BP_BlocksCounter.TotalScore` (`/Game/Blueprints/GI_ArkanoidGameInstance.Score` _asgi_arkanoid_game_instance) _bp_blockscounter)
  (bind _outactors (`GameplayStatics.GetAllActorsOfClass` "/Game/Blueprints/BP_Block_Child.BP_Block_Child_C"))
  (bind _output_get (set `self.BlocksArray` _outactors))
  (set `/Game/Blueprints/ActorComponents/BP_BlocksCounter.BlocksCounter` (`KismetArrayLibrary.Array_Length` _output_get) _bp_blockscounter)
  (set `self.DefaultRacketScale` (`SceneComponent.RelativeScale3D` (`self.Cube`))))

(fn `LevelCompleted`
  (bind _returnvalue (`GameplayStatics.GetPlayerController` (`self.Player Index`)))
  (`Widget.SetVisibility` (`self.Hud`) "Collapsed")
  (bind _returnvalue_2 (`|CreateWidget` "/Game/Blueprints/UI/W_LevelWin.W_LevelWin_C" _returnvalue))
  (`UserWidget.AddToViewport` _returnvalue_2 0)
  (`WidgetBlueprintLibrary.SetInputMode_UIOnlyEx` _returnvalue _returnvalue_2 "LockOnCapture")
  (set `PlayerController.bShowMouseCursor` true _returnvalue)
  (`GameplayStatics.SetGamePaused` true))

(fn `RespawnBall`
  (bind _outactors (`GameplayStatics.GetAllActorsOfClass` "/Game/Blueprints/BP_Ball.BP_Ball_C"))
  (bind _output_get (set `self.BallsCount` (- (`KismetArrayLibrary.Array_Length` _outactors) 1)))
  (if (== _output_get 0)
    (`/Game/Blueprints/ActorComponents/BP_LivesComponent.Sub` (`self.BP_LivesComponent`))
    (`GameplayStatics.PlaySoundAtLocation` "/Game/Blueprints/Audio/S_RespawnRacket_Cue.S_RespawnRacket_Cue" (`self.K2_GetActorLocation`) (struct) 1.0 1.0 0.0 null null null)
    (bind _outactors_2 (`GameplayStatics.GetAllActorsOfClass` "/Game/Blueprints/Bonuses/BP_Bonus.BP_Bonus_C"))
    (`self.K2_DestroyActor` _outactors_2)
    (bind _cube (`self.Cube`)
      (:`then`
        (`SceneComponent.SetWorldScale3D` _cube (`self.DefaultRacketScale`))
        (`self.SpawnBall`))
      (:`else`))))

(fn `SetGameInstance`
  (bind _asgi_arkanoid_game_instance (cast `/Game/Blueprints/GI_ArkanoidGameInstance` (`GameplayStatics.GetGameInstance`)))
  (set `/Game/Blueprints/GI_ArkanoidGameInstance.Lives` (`/Game/Blueprints/ActorComponents/BP_LivesComponent.Lives` (`self.BP_LivesComponent`)) _asgi_arkanoid_game_instance)
  (set `/Game/Blueprints/GI_ArkanoidGameInstance.Score` (`/Game/Blueprints/ActorComponents/BP_BlocksCounter.TotalScore` (`self.BP_BlocksCounter`)) _asgi_arkanoid_game_instance))

(fn `ShootBullets`
  (`self.Cube`
    (:`then`
      (if (<= (`self.BulletsCounter`) 7)
        (`|SpawnActorFromClass` "/Game/Blueprints/BP_Bullet.BP_Bullet_C" (`KismetMathLibrary.MakeTransform` (`SceneComponent.K2_GetComponentLocation` (`self.LaserRight`)) (struct :`Roll` 90.0) (0.3 0.3 0.7)) "AlwaysSpawn" "OverrideRootScale" null null)
        (`|SpawnActorFromClass` "/Game/Blueprints/BP_Bullet.BP_Bullet_C" (`KismetMathLibrary.MakeTransform` (`SceneComponent.K2_GetComponentLocation` (`self.LaserLeft`)) (struct :`Roll` 90.0) (0.3 0.3 0.7)) "AlwaysSpawn" "OverrideRootScale" null null)
        (`/Engine/EditorBlueprintResources/StandardMacros.IncrementInt` (`self.BulletsCounter`))
        (else
          (`KismetSystemLibrary.K2_ClearAndInvalidateTimerHandle` (`self.TimerHandle`))
          (set `self.BulletsCounter` 0))))
    (:`else`)))

(fn `SpawnBall`
  (`self.Cube`
    (:`then`
      (bind _returnvalue (`|SpawnActorFromClass` "/Game/Blueprints/BP_Ball.BP_Ball_C" (`KismetMathLibrary.MakeTransform` (`SceneComponent.K2_GetComponentLocation` (`self.Sphere`))) "AlwaysSpawn" "OverrideRootScale" null null))
      (set `self.PlayingBall` _returnvalue)
      (bind _playingball (`self.PlayingBall`)
        (:`then`
          (`SceneComponent.K2_AttachToComponent` (`Actor.RootComponent` _playingball) (`self.Cube`) "None" "KeepWorld" "KeepWorld" "KeepWorld" false)
          (add `/Game/Blueprints/BP_Ball.OnBallDead` _playingball (`|CreateDelegate` :!event `RespawnBall`))
          (return))
        (:`else`)))
    (:`else`)))

(fn `SpawnBonusBall`
  (`self.Cube`
    (:`then`
      (bind _returnvalue (`|SpawnActorFromClass` "/Game/Blueprints/BP_Ball.BP_Ball_C" (`KismetMathLibrary.MakeTransform` (`SceneComponent.K2_GetComponentLocation` (`self.Sphere`))) "AlwaysSpawn" "OverrideRootScale" null null))
      (set `self.PlayingBall` _returnvalue)
      (bind _playingball (`self.PlayingBall`)
        (:`then`
          (`SceneComponent.K2_AttachToComponent` (`Actor.RootComponent` _playingball) (`self.Cube`) "None" "KeepWorld" "KeepWorld" "KeepWorld" false)
          (`self.K2_DetachFromActor` _playingball "KeepWorld" "KeepWorld" "KeepWorld")
          (`self.OnPushBall`)
          (add `/Game/Blueprints/BP_Ball.OnBallDead` _playingball (`|CreateDelegate` :!event `RespawnBall`))
          (return))
        (:`else`)))
    (:`else`)))

(fn `SpawnBullets`
  (bind _returnvalue (`KismetSystemLibrary.K2_SetTimerDelegate` (`|CreateDelegate` :!event `ShootBullets`) (`self.BulletsTimer`) true))
  (set `self.TimerHandle` _returnvalue))

(fn `UserConstructionScript`)