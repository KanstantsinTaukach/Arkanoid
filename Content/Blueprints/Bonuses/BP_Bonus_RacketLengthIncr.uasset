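; Racket length bonus pickup that, when activated, plays a pickup sound and widens the player's BP_Racket by multiplying its actor X scale by 1.1.
; If the racket's absolute X position is at or beyond RacketLocationForBonus, it first shifts the racket a fixed step toward X zero and raises that threshold by a tenth of the default X scale.
; An unused branch scales the Cube component instead of the actor.
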(fn `Activate`
  (`GameplayStatics.PlaySoundAtLocation` "/Game/Blueprints/Audio/S_TakeBonus_Cue.S_TakeBonus_Cue" (`self.K2_GetActorLocation`) (struct) 1.0 1.0 0.0 null null null)
  (bind _asbp_racket (cast `/Game/Blueprints/BP_Racket` (`GameplayStatics.GetPlayerPawn` 0)))
  (bind _returnvalue_x (`KismetMathLibrary.BreakVector` (`self.K2_GetActorLocation` _asbp_racket)))
  (bind _racketlocationforbonus_x (`KismetMathLibrary.BreakVector` (`/Game/Blueprints/BP_Racket.RacketLocationForBonus` _asbp_racket)))
  (if (>= (`KismetMathLibrary.Abs` _returnvalue_x) _racketlocationforbonus_x)
    (bind (_returnvalue_x_2 _returnvalue_y _returnvalue_z) (`KismetMathLibrary.BreakVector` (`self.K2_GetActorLocation` _asbp_racket)))
    (`self.K2_SetActorLocation` _asbp_racket (`KismetMathLibrary.MakeVector` (+ _returnvalue_x_2 (`KismetMathLibrary.SelectFloat` -25.0 25.0 (> _returnvalue_x_2 0.0))) _returnvalue_y _returnvalue_z) false false)
    (bind _racketlocationforbonus_x_2 (`KismetMathLibrary.BreakVector` (`/Game/Blueprints/BP_Racket.RacketLocationForBonus` _asbp_racket)))
    (bind _defaultracketscale_x (`KismetMathLibrary.BreakVector` (`/Game/Blueprints/BP_Racket.DefaultRacketScale` _asbp_racket)))
    (set `/Game/Blueprints/BP_Racket.RacketLocationForBonus` (`KismetMathLibrary.MakeVector` (+ _racketlocationforbonus_x_2 (- (* _defaultracketscale_x 1.1) _defaultracketscale_x))) _asbp_racket))
  (bind (_returnvalue_x_3 _returnvalue_y_2 _returnvalue_z_2) (`KismetMathLibrary.BreakVector` (`self.GetActorScale3D` _asbp_racket)))
  (`self.SetActorScale3D` _asbp_racket (`KismetMathLibrary.MakeVector` (* _returnvalue_x_3 1.1) _returnvalue_y_2 _returnvalue_z_2)))

(fn `UserConstructionScript`
  (`parent.UserConstructionScript`))