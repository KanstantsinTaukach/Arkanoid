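; BP_Bonus_RacketLengthDecr is a penalty pickup that shortens the player's racket.
; Activate plays an invalid-action sound at the bonus location, then casts the player pawn to BP_Racket.
; It multiplies the X scale of the racket's Cube by 0.85, so repeated activations compound with no lower limit or revert in this Blueprint.
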(fn `Activate`
  (`GameplayStatics.PlaySoundAtLocation` "/Game/Blueprints/Audio/S_InvalidAction_Cue.S_InvalidAction_Cue" (`self.K2_GetActorLocation`) (struct) 1.0 1.0 0.0 null null null)
  (bind _asbp_racket (cast `/Game/Blueprints/BP_Racket` (`GameplayStatics.GetPlayerPawn` 0)))
  (bind _cube (`/Game/Blueprints/BP_Racket.Cube` _asbp_racket))
  (bind (_relativescale3d_x _relativescale3d_y _relativescale3d_z) (`KismetMathLibrary.BreakVector` (`SceneComponent.RelativeScale3D` _cube)))
  (`SceneComponent.SetRelativeScale3D` _cube (`KismetMathLibrary.MakeVector` (* _relativescale3d_x 0.85) _relativescale3d_y _relativescale3d_z)))

(fn `UserConstructionScript`
  (`parent.UserConstructionScript`))