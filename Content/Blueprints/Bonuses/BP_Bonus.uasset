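; BP_Bonus is a bonus pickup actor that moves along Y once dropped and is collected by the racket.
; Its OnDropBonus event starts a timeline that offsets the actor by BonusDirection.Y scaled by the track value.
; Overlapping BP_Racket calls Activate, empty here as an apparent hook for child bonuses, then destroys the actor.
; Overlapping a KillZVolume destroys it without activation.
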(event `self.ReceiveBeginPlay`
  (add `self.OnDropBonus` (delegate `OnDropBonus_Event`)))

(event `OnDropBonus_Event`
  (bind (_bonusdirection_x _bonusdirection_y) (`KismetMathLibrary.BreakVector` (`self.BonusDirection`)))
  (bind (_direction _newtrack_0) (`Timeline|BonusDirectionY`)
    (:`Update`
      (bind (_returnvalue_x _returnvalue_y) (`KismetMathLibrary.BreakVector` (* (`KismetMathLibrary.MakeVector` 0.0 _bonusdirection_y) _newtrack_0)))
      (`self.K2_AddActorWorldOffset` (`KismetMathLibrary.MakeVector` 0.0 _returnvalue_y)))))

(event `self.Cube.OnComponentBeginOverlap`
  (params (OverlappedComponent :type "PrimitiveComponent Object Reference") (OtherActor :type "Actor Object Reference") (OtherComp :type "PrimitiveComponent Object Reference") (OtherBodyIndex :type Integer) (bFromSweep :type Boolean) (SweepResult :type "HitResult Structure (by ref)"))
  ;[1 1 1] Bonus Component Overlap
  (cast `/Game/Blueprints/BP_Racket` OtherActor
    (:`then`
      (`self.Activate`))
    (:`CastFailed`
      (cast `KillZVolume` OtherActor)))
  (`self.K2_DestroyActor`))

(fn `Activate`)

(fn `UserConstructionScript`)