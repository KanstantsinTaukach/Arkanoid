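; Actor component that keeps a lives counter for its owning actor.
; Add and Sub change the count by one through a shared Update function.
; Update fires OnLivesUpdate before storing the new value, then fires OnLivesEnd if IsDead finds the count at zero or below.
; It is driven entirely by these calls, with no active BeginPlay or Tick logic.
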(fn `Add`
  (`self.Update` (+ (`self.Lives`) 1)))

(fn `IsDead`
  (returns (ReturnValue :type Boolean))
  (return (<= (`self.Lives`) 0)))

(fn `Sub`
  (`self.Update` (- (`self.Lives`) 1)))

(fn `Update`
  (params (Lives :type Integer))
  (`self.OnLivesUpdate`)
  (set `self.Lives` Lives)
  (if (`self.IsDead`)
    (`self.OnLivesEnd`)))