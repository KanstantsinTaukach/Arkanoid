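; BP_BlocksCounter is an actor component that tracks the remaining block count and the accumulated score.
; SubBlock adds a score to the total and decrements the count through Update.
; Update fires the blocks-update dispatcher before storing the new values, then fires the blocks-end dispatcher when IsEmpty finds the count at zero or below.
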(fn `IsEmpty`
  (returns (ReturnValue :type Boolean))
  (return (<= (`self.BlocksCounter`) 0)))

(fn `SubBlock`
  (params (score :type Integer))
  (`self.Update` (+ score (`self.TotalScore`)) (- (`self.BlocksCounter`) 1)))

(fn `Update`
  (params (BlocksScore :type Integer) (BlocksQuantity :type Integer))
  (`self.OnBlocksUpdate`)
  (set `self.TotalScore` BlocksScore)
  (set `self.BlocksCounter` BlocksQuantity)
  (if (`self.IsEmpty`)
    (`self.OnBlocksEnd`)))