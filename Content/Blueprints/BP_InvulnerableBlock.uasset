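; BP_InvulnerableBlock is a block actor that builds a flat grid of static meshes in its construction script.
; Nested loops over X and Y add one static mesh component per cell, offset by the index times Padding at zero local height.
; The graph holds only this layout step, with no damage or invulnerability logic.
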(fn `UserConstructionScript`
  (for _index (range (`self.X`))
    (for _index_2 (range (`self.Y`))
      (`AddComponent|NODE_AddStaticMeshComponent-6` :`RelativeTransform` (`KismetMathLibrary.MakeTransform` (`KismetMathLibrary.MakeVector` (`KismetMathLibrary.Conv_IntToDouble` (* _index (`self.Padding`))) (`KismetMathLibrary.Conv_IntToDouble` (* _index_2 (`self.Padding`))) 0.0))))))