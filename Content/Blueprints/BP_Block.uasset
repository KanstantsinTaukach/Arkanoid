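; Breakable block that loses one of its four lives each time a BP_Ball hits it.
; A lives component tracks damage and exposes update and death events, bound at BeginPlay.
; Helper functions cycle the cube through a material array with debug prints, and destroy the block with a weighted random chance to spawn a BP_Bonus drop.
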(event `self.ReceiveBeginPlay`
  (`self.InitializeBlockLives`)
  (`self.Binds`))

(event `self.ReceiveHit`
  (params (MyComp :type "PrimitiveComponent Object Reference") (Other :type "Actor Object Reference") (OtherComp :type "PrimitiveComponent Object Reference") (bSelfMoved :type Boolean) (HitLocation :type "Vector Structure") (HitNormal :type "Vector Structure") (NormalImpulse :type "Vector Structure") (Hit :type "HitResult Structure (by ref)"))
  (cast `/Game/Blueprints/BP_Ball` Other)
  (`/Game/Blueprints/ActorComponents/BP_LivesComponent.Sub` (`self.BP_LivesComponent`)))

(fn `Binds`
  (bind _bp_livescomponent (`self.BP_LivesComponent`))
  (add `/Game/Blueprints/ActorComponents/BP_LivesComponent.OnLivesUpdate` _bp_livescomponent (`|CreateDelegate` :!event `ChangeMaterial`))
  (add `/Game/Blueprints/ActorComponents/BP_LivesComponent.OnDeath` _bp_livescomponent (`|CreateDelegate` :!event `DestroyBlock`)))

(fn `ChangeMaterial`
  (if (< (`self.MaterialIterator`) (- (`KismetArrayLibrary.Array_Length` (`self.BlockMaterials`)) 1))
    (bind _result (`/Engine/EditorBlueprintResources/StandardMacros.IncrementInt` (`self.MaterialIterator`))
      (:`  `
        (`PrimitiveComponent.SetMaterial` (`self.Cube`) 0 (`|GetArrayItem` (`self.BlockMaterials`) _result))
        (`KismetSystemLibrary.PrintString` (`KismetStringLibrary.Concat_StrStr` "True: lives left - " (`KismetStringLibrary.Conv_IntToString` (- (`/Game/Blueprints/ActorComponents/BP_LivesComponent.Lives` (`self.BP_LivesComponent`)) 1)) " Iterator - " (`KismetStringLibrary.Conv_IntToString` (`self.MaterialIterator`))) true true (struct :`R` 1.0 :`G` 0.005986 :`B` 0.095644 :`A` 1.0) 7.0)))
    (else
      (bind _output_get (set `self.MaterialIterator` 0))
      (`PrimitiveComponent.SetMaterial` (`self.Cube`) 0 (`|GetArrayItem` (`self.BlockMaterials`) _output_get))
      (`KismetSystemLibrary.PrintString` (`KismetStringLibrary.Concat_StrStr` "False: lives left - " (`KismetStringLibrary.Conv_IntToString` (- (`/Game/Blueprints/ActorComponents/BP_LivesComponent.Lives` (`self.BP_LivesComponent`)) 1)) " Iterator - " (`KismetStringLibrary.Conv_IntToString` (`self.MaterialIterator`))) true true (struct :`R` 1.0 :`G` 0.808392 :`A` 1.0) 7.0))))

(fn `DestroyBlock`
  (`self.DropBonus`)
  (`self.K2_DestroyActor`))

(fn `DropBonus`
  (if (`KismetMathLibrary.RandomBoolWithWeight` 0.3)
    (bind _returnvalue (`|SpawnActorFromClass` "/Game/Blueprints/BP_Bonus.BP_Bonus_C" (`KismetMathLibrary.MakeTransform` (`SceneComponent.K2_GetComponentLocation` (`self.Cube`)) (struct) (0.8 0.8 0.8)) "AlwaysSpawn" "OverrideRootScale" null null))
    (bind _output_get (set `self.DroppingBonus` _returnvalue))
    (`/Game/Blueprints/BP_Bonus.OnDropBonus` _output_get)))

(fn `InitializeBlockLives`
  (set `/Game/Blueprints/ActorComponents/BP_LivesComponent.Lives` 4 (`self.BP_LivesComponent`)))

(fn `UserConstructionScript`)