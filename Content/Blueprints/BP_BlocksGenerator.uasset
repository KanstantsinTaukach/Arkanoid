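; BP_BlocksGenerator lays out a configurable X by Y grid of blocks with uniform padding.
; The construction script builds a preview grid of static mesh components and stores them in BlocksArray.
; On BeginPlay it destroys those components and spawns BP_Block_Child actors offset from the generator's XY location at a fixed world height, passing BlockLives to each.
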(event `self.ReceiveBeginPlay`
  (bind (_returnvalue_x _returnvalue_y) (`KismetMathLibrary.BreakVector` (`self.K2_GetActorLocation`)))
  (bind _returnvalue_x_2 (`KismetMathLibrary.BreakVector` (`self.K2_GetActorLocation`)))
  (for _array_element (`self.BlocksArray`)
    (`ActorComponent.K2_DestroyComponent` _array_element))
  (for _index (range (`self.X`))
    (for _index_2 (range (`self.Y`))
      (`|SpawnActorFromClass` "/Game/Blueprints/BP_Block_Child.BP_Block_Child_C" (`KismetMathLibrary.MakeTransform` (`KismetMathLibrary.MakeVector` (+ (`KismetMathLibrary.Conv_IntToDouble` (* _index (`self.Padding`))) _returnvalue_x_2) (+ (`KismetMathLibrary.Conv_IntToDouble` (* _index_2 (`self.Padding`))) _returnvalue_y) 71.0)) "AlwaysSpawn" "OverrideRootScale" null (`self.Block Lives`) null))))

(fn `UserConstructionScript`
  (for _index (range (`self.X`))
    (for _index_2 (range (`self.Y`))
      (bind _returnvalue (`AddComponent|NODE_AddStaticMeshComponent-0` :`RelativeTransform` (`KismetMathLibrary.MakeTransform` (`KismetMathLibrary.MakeVector` (`KismetMathLibrary.Conv_IntToDouble` (* _index (`self.Padding`))) (`KismetMathLibrary.Conv_IntToDouble` (* _index_2 (`self.Padding`))) 50.0))))
      (`KismetArrayLibrary.Array_Add` (`self.BlocksArray`) _returnvalue))))